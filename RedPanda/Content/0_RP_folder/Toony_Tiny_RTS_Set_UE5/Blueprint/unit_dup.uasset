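; Modular unit Blueprint from the Toony Tiny RTS set that assembles its appearance from selectable body, head and material options.
; The construction script picks body and head skeletal meshes from the Body and Heads collections using BodyMesh and HeadMesh.
; EnemyClass selects one material from Material1, applied to the first slot of both meshes.
; The event graph holds only disabled placeholder events, so the Blueprint adds no runtime logic.
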(fn `UserConstructionScript`
  (bind _output (`|GetArrayItem` (`self.material1`) (`self.enemy class`)))
  (`SkeletalMeshComponent.SetSkeletalMeshAsset` (`self.SkeletalMeshComponent`) (`|GetArrayItem` (`self.body`) (`self.body mesh`)))
  (`PrimitiveComponent.SetMaterial` (`self.SkeletalMeshComponent`) 0 _output)
  (`PrimitiveComponent.SetMaterial` (`self.Head`) 0 _output)
  (`SkeletalMeshComponent.SetSkeletalMeshAsset` (`self.Head`) (`|GetArrayItem` (`self.heads`) (`self.head mesh`))))