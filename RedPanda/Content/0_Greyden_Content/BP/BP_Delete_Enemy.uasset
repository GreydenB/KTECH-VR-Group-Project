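; BP_Delete_Enemy is a kill-zone actor that damages the Castle when enemies enter it.
; The Cube's begin-overlap event filters for the Enemy tag, then checks type tags to set AttackDMG.
; Goblin, Orc and Cyclops pass increasing damage to Castle's Hit function.
; The Sphere branch only sets AttackDMG without calling Hit, and despite the asset's name nothing here destroys the enemy.
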(event `self.Cube.OnComponentBeginOverlap`
  (params (OverlappedComponent :type "PrimitiveComponent Object Reference") (OtherActor :type "Actor Object Reference") (OtherComp :type "PrimitiveComponent Object Reference") (OtherBodyIndex :type Integer) (bFromSweep :type Boolean) (SweepResult :type "HitResult Structure (by ref)"))
  ;[0.8385 0.1791 0.1791] Detects is enemy is in kill zone
  (if (`self.ActorHasTag` OtherActor "Enemy")
    (if (`self.ActorHasTag` OtherActor "Goblin")
      (set `self.Attack DMG` 1)
      (`/Game/0_Greyden_Content/BP/BP_Castle.Hit` (`self.Castle`) (`self.Attack DMG`) :!label _label)
      (elif (`self.ActorHasTag` OtherActor "Orc")
        (set `self.Attack DMG` 2)
        (goto _label)
        (elif (`self.ActorHasTag` OtherActor "Cyclops")
          (set `self.Attack DMG` 3)
          (goto _label)
          (elif (`self.ActorHasTag` OtherActor "Sphere")
            (set `self.Attack DMG` 15)))))))

(fn `UserConstructionScript`)