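; Enemy spawner for a VR castle wave game that spawns random goblins, orcs or cyclopes around itself.
; Three wave events set difficulty, update the VR pawn's status and start a countdown alongside a self-recalling, randomly delayed spawn loop with chance-based spawns.
; When time runs out, a final loop spawns a guaranteed batch, then asks the castle whether the final wave is over.
; Do-once gates trigger the castle's enemy check.
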(event `Wave 1`
  (params (Time :type Integer))
  ;[1 0 0.05706] Wave 1
  (set `self.Spawn_Time` Time)
  (set `self.Final Spawn Amount` 2)
  (set `self.Time Between Spawns Max` 5)
  (set `self.Time Between Spawns Min` 3)
  (set `self.Spawn_Chance_Original` 8)
  (`self.Spawn_Wave`)
  (`self.Countdown`)
  (bind _asvrpawn (cast `/Game/VRTemplate/Blueprints/VRPawn` (`GameplayStatics.GetPlayerPawn` 0)))
  (set `/Game/VRTemplate/Blueprints/VRPawn.Status` "Wave 1" _asvrpawn))

(event `Wave 2`
  (params (Time :type Integer))
  ;[0.9731 1 0] Wave 2
  (set `self.Spawn_Time` Time)
  (set `self.Final Spawn Amount` 3)
  (set `self.Time Between Spawns Max` 4)
  (set `self.Time Between Spawns Min` 3)
  (set `self.Spawn_Chance_Original` 6)
  (set `self.Spawn Chance` 1)
  (`self.Spawn_Wave`)
  (`self.Countdown`)
  (bind _asvrpawn (cast `/Game/VRTemplate/Blueprints/VRPawn` (`GameplayStatics.GetPlayerPawn` 0)))
  (set `/Game/VRTemplate/Blueprints/VRPawn.Status` "Wave 2" _asvrpawn))

(event `Wave 3`
  (params (Time :type Integer))
  ;[0 0.1683 1] Wave 3
  (set `self.Spawn_Time` Time)
  (set `self.Final Spawn Amount` 5)
  (set `self.Time Between Spawns Max` 4)
  (set `self.Time Between Spawns Min` 2)
  (set `self.Spawn_Chance_Original` 4)
  (set `self.Spawn Chance` 1)
  (`self.Spawn_Wave`)
  (`self.Countdown`)
  (bind _asvrpawn (cast `/Game/VRTemplate/Blueprints/VRPawn` (`GameplayStatics.GetPlayerPawn` 0)))
  (set `/Game/VRTemplate/Blueprints/VRPawn.Status` "Wave 3" _asvrpawn))

(event `Countdown`
  ;[0.3397 0.9302 1] Countdown
  (`/Engine/EditorBlueprintResources/StandardMacros.DecrementInt` (`self.Spawn_Time`)
    (:`  `
      (`KismetSystemLibrary.Delay` 1.0)
      (`self.Countdown`))))

(event `Spawn_Wave`
  (bind (_returnvalue_x _returnvalue_y _returnvalue_z) (`KismetMathLibrary.BreakVector` (`self.K2_GetActorLocation`)))
  ;[0.04746 1 0.9103] Spawns enemys for wave
  (if (== (`self.Spawn Chance`) (`KismetMathLibrary.RandomIntegerInRange` 1 (`self.Spawn Chance`)))
    ;;[1 1 1] Spawns Enemy in random location within range
    (`|SpawnActorFromClass` (select `int` (`KismetMathLibrary.RandomIntegerInRange` 0 2) :`0` "/Game/0_Greyden_Content/AI/AI_Goblin.AI_Goblin_C" :`1` "/Game/0_Greyden_Content/AI/AI_Orc.AI_Orc_C" :`2` "/Game/0_Greyden_Content/AI/AI_Cyclops.AI_Cyclops_C" :!type "Actor Class Reference") (`KismetMathLibrary.MakeTransform` (`KismetMathLibrary.MakeVector` (+ _returnvalue_x (`KismetMathLibrary.RandomIntegerInRange` -1500 1500)) (+ _returnvalue_y (`KismetMathLibrary.RandomIntegerInRange` -1500 1500)) _returnvalue_z)) "Undefined" "MultiplyWithRoot" null null))
  (`KismetSystemLibrary.Delay` (`KismetMathLibrary.Conv_IntToDouble` (`KismetMathLibrary.RandomIntegerInRange` (`self.Time Between Spawns Min`) (`self.Time Between Spawns Max`))))
  ;;[1 0.8413 0.08369] Checks time left
  (if (>= (`self.Spawn_Time`) 0)
    ;;[1 0 0.7921] Loops Spawn Wave 1 for Spawn amount
    (`self.Spawn_Wave`)
    ;;[1 1 1] Initiates Check Enemy
    (`/Engine/EditorBlueprintResources/StandardMacros.DoOnce` false :!label _label
      (:`Completed`
        (`/Game/0_Greyden_Content/BP/BP_Castle.Check_Enemy` (`self.Castle_Ref`))
        ;;[0.1906 1 0.07532] Set Spawn chance to non guaranteed
        (set `self.Spawn Chance` (`self.Spawn_Chance_Original`))))
    (else
      (`self.Wave_F`)
      (goto _label :!via `Reset`))))

(event `Wave_F`
  (bind (_returnvalue_x _returnvalue_y _returnvalue_z) (`KismetMathLibrary.BreakVector` (`self.K2_GetActorLocation`)))
  ;[0.1332 1 0.9403] Final of wave
  (`|SpawnActorFromClass` (select `int` (`KismetMathLibrary.RandomIntegerInRange` 0 2) :`0` "/Game/0_Greyden_Content/AI/AI_Goblin.AI_Goblin_C" :`1` "/Game/0_Greyden_Content/AI/AI_Orc.AI_Orc_C" :`2` "/Game/0_Greyden_Content/AI/AI_Cyclops.AI_Cyclops_C" :!type "Actor Class Reference") (`KismetMathLibrary.MakeTransform` (`KismetMathLibrary.MakeVector` (+ _returnvalue_x (`KismetMathLibrary.RandomIntegerInRange` -1500 1500)) (+ _returnvalue_y (`KismetMathLibrary.RandomIntegerInRange` -1500 1500)) _returnvalue_z)) "Undefined" "MultiplyWithRoot" null null)
  (`KismetSystemLibrary.Delay` (`KismetMathLibrary.RandomFloatInRange` 2.0 3.0))
  ;;[1 0.8413 0.08369] Checks number of spawns left
  (if (!= 0 (`self.Final Spawn Amount`))
    ;;[1 0.8213 0] Subtracts from amount of spawns left
    (set `self.Final Spawn Amount` (- (`self.Final Spawn Amount`) 1))
    ;;[1 0 0.7921] Loops Spawn Wave 1 F for Final Spawn amount
    (`self.Wave_F`)
    ;;[1 1 1] Initiates Check Enemy
    (`/Engine/EditorBlueprintResources/StandardMacros.DoOnce` false :!label _label_2
      (:`Completed`
        (`/Game/0_Greyden_Content/BP/BP_Castle.Check_Enemy` (`self.Castle_Ref`))))
    (else
      (`/Game/0_Greyden_Content/BP/BP_Castle.Is final wave over?` (`self.Castle_Ref`))
      (goto _label_2 :!via `Reset`))))

(fn `UserConstructionScript`)