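; BP_Castle is the defended castle that also directs a three-wave VR game, ending in a win or loss level.
; Each wave passes rising duration and catapult settings to all spawners and updates the VRPawn's status and timer.
; A delayed enemy check advances waves or declares victory once eight spawners report done and no "Enemy"-tagged actors remain.
; Hits reduce castle HP, triggering game over at zero, otherwise updating the pawn and playing a sound.
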(event `Activate Wave 1`
  ;[1 0.08013 0] Activate Wave 1
  (bind _asvrpawn (cast `/Game/VRTemplate/Blueprints/VRPawn` (`GameplayStatics.GetPlayerPawn` 0)))
  (set `/Game/VRTemplate/Blueprints/VRPawn.Status` "Starting Wave 1 Soon" _asvrpawn)
  (`KismetSystemLibrary.Delay` 5.0)
  (bind _output_get (set `self.Wave Time` 120))
  (`/Game/VRTemplate/Blueprints/VRPawn.Set Wave Timer` _asvrpawn _output_get)
  (set `self.Max Catapults` 2)
  (set `self.Catapult Spawn Chance` 8)
  (bind _outactors (`GameplayStatics.GetAllActorsOfClass` "/Game/0_Greyden_Content/BP/BP_Spawner.BP_Spawner_C"))
  (`/Game/0_Greyden_Content/BP/BP_Spawner.Wave 1` _outactors (`self.Wave Time`))
  (bind _outactors_2 (`GameplayStatics.GetAllActorsOfClass` "/Game/0_Greyden_Content/BP/BP_Catapult_Spawner.BP_Catapult_Spawner_C"))
  (`/Game/0_Greyden_Content/BP/BP_Catapult_Spawner.Spawn_Catapults` _outactors_2 (`self.Max Catapults`) (`self.Catapult Spawn Chance`) (`self.Wave Time`)))

(event `Is final wave over?`
  (bind _spawners_done (`self.Spawners Done`))
  ;[1 1 1] Checks if all waves are over
  (`/Engine/EditorBlueprintResources/StandardMacros.IncrementInt` _spawners_done
    (:`  `
      (if (== 8 _spawners_done)
        (set `self.WavesOver` true)))))

(event `Check_Enemy`
  ;[1 0 0] Checks Enemys in level every 5 seconds
  (`KismetSystemLibrary.Delay` 5.0)
  (bind _outactors (`GameplayStatics.GetAllActorsWithTag` "Enemy"))
  (set `self.Number_Of_Enemies` (`KismetArrayLibrary.Array_Length` _outactors))
  (if (<= (`self.Number_Of_Enemies`) 0)
    (if (`self.WavesOver`)
      ;[1 0.4717 0] Activate Wave 2
      (if (== 1 (`self.Wave Number`))
        (bind _asvrpawn (cast `/Game/VRTemplate/Blueprints/VRPawn` (`GameplayStatics.GetPlayerPawn` 0)))
        (set `/Game/VRTemplate/Blueprints/VRPawn.Status` "Starting Wave 2 Soon" _asvrpawn)
        (`KismetSystemLibrary.Delay` 30.0)
        (set `self.Spawners done` 0)
        (`/Engine/EditorBlueprintResources/StandardMacros.IncrementInt` (`self.Wave Number`)
          (:`  `
            (set `self.WavesOver` false)
            (bind _output_get (set `self.Wave Time` 180))
            (`/Game/VRTemplate/Blueprints/VRPawn.Set Wave Timer` _asvrpawn _output_get)
            (set `self.Max Catapults` 3)
            (set `self.Catapult Spawn Chance` 6)
            (bind _outactors_2 (`GameplayStatics.GetAllActorsOfClass` "/Game/0_Greyden_Content/BP/BP_Spawner.BP_Spawner_C"))
            (`/Game/0_Greyden_Content/BP/BP_Spawner.Wave 2` _outactors_2 (`self.Wave Time`))
            (bind _outactors_3 (`GameplayStatics.GetAllActorsOfClass` "/Game/0_Greyden_Content/BP/BP_Catapult_Spawner.BP_Catapult_Spawner_C"))
            (`/Game/0_Greyden_Content/BP/BP_Catapult_Spawner.Spawn_Catapults` _outactors_3 (`self.Max Catapults`) (`self.Catapult Spawn Chance`) (`self.Wave Time`))))
        (else
          ;[1 0.8872 0] Activate Wave 3
          (if (== 2 (`self.Wave Number`))
            (bind _asvrpawn_2 (cast `/Game/VRTemplate/Blueprints/VRPawn` (`GameplayStatics.GetPlayerPawn` 0)))
            (set `/Game/VRTemplate/Blueprints/VRPawn.Status` "Starting Wave 3 Soon" _asvrpawn_2)
            (`KismetSystemLibrary.Delay` 30.0)
            (set `self.Spawners done` 0)
            (`/Engine/EditorBlueprintResources/StandardMacros.IncrementInt` (`self.Wave Number`)
              (:`  `
                (set `self.WavesOver` false)
                (bind _output_get_2 (set `self.Wave Time` 240))
                (`/Game/VRTemplate/Blueprints/VRPawn.Set Wave Timer` _asvrpawn_2 _output_get_2)
                (set `self.Max Catapults` 4)
                (set `self.Catapult Spawn Chance` 4)
                (bind _outactors_4 (`GameplayStatics.GetAllActorsOfClass` "/Game/0_Greyden_Content/BP/BP_Spawner.BP_Spawner_C"))
                (`/Game/0_Greyden_Content/BP/BP_Spawner.Wave 3` _outactors_4 (`self.Wave Time`))
                (bind _outactors_5 (`GameplayStatics.GetAllActorsOfClass` "/Game/0_Greyden_Content/BP/BP_Catapult_Spawner.BP_Catapult_Spawner_C"))
                (`/Game/0_Greyden_Content/BP/BP_Catapult_Spawner.Spawn_Catapults` _outactors_5 (`self.Max Catapults`) (`self.Catapult Spawn Chance`) (`self.Wave Time`))))
            (else
              ;[0.6123 1 0] Win Game
              (if (== 3 (`self.Wave Number`))
                (bind _asvrpawn_3 (cast `/Game/VRTemplate/Blueprints/VRPawn` (`GameplayStatics.GetPlayerPawn` 0)))
                (set `/Game/VRTemplate/Blueprints/VRPawn.Status` "Game Won" _asvrpawn_3)
                (`GameplayStatics.OpenLevel` "EndRoom_M"))))))
      (else
        (`KismetSystemLibrary.PrintString` "Waves not over")
        (`self.Check_Enemy` :!label _label)))
    (else
      (goto _label))))

(event `Hit`
  (params (Damage :type Integer))
  (bind _castle_hp (`self.Castle HP`))
  ;[0.9407 1 0.431] After Castle is hit
  (set `self.Castle HP` (- _castle_hp Damage))
  (if (<= _castle_hp 0)
    (bind _asvrpawn (cast `/Game/VRTemplate/Blueprints/VRPawn` (`GameplayStatics.GetPlayerPawn` 0)))
    (set `/Game/VRTemplate/Blueprints/VRPawn.Status` "Game Over" _asvrpawn)
    (`GameplayStatics.OpenLevel` "EndRoom_Loss")
    (else
      (bind _asvrpawn_2 (cast `/Game/VRTemplate/Blueprints/VRPawn` (`GameplayStatics.GetPlayerPawn` 0)))
      (set `/Game/VRTemplate/Blueprints/VRPawn.Castle HP Pawn` (`self.Castle HP`) _asvrpawn_2)
      (`self.Hit_Sound`))))

(event `Hit_Sound`
  (`KismetSystemLibrary.Delay` 0.5)
  (`GameplayStatics.PlaySoundAtLocation` "/Game/0_Greyden_Content/Sound/retro-explode-1-236678.retro-explode-1-236678" (`self.K2_GetActorLocation`) (struct) 1.0 1.0 0.0 null null null null))

(fn `UserConstructionScript`)