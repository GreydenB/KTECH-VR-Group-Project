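; Catapult spawner that places AI_Catapult actors at random horizontal offsets around itself during a timed wave.
; Spawn_Catapults stores the wave settings, then starts a self-repeating one-second countdown and a randomly delayed spawn loop.
; Each pass has a one-in-CatapultSpawnChance roll, capped by the world count of "Catapult"-tagged actors.
; Once time runs out, a final briefly delayed spawn skips the roll but respects the cap.
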(event `Countdown`
  (`/Engine/EditorBlueprintResources/StandardMacros.DecrementInt` (`self.Wave_Time`)
    (:`  `
      (`KismetSystemLibrary.Delay` 1.0)
      (`self.Countdown`))))

(event `Spawn_Catapults`
  (params (MaxCatapults :type Integer) (CatapultSpawnChance :type Integer) (`Wave Time` :type Integer))
  (set `self.Wave_Time` `Wave Time`)
  (set `self.Catapult Spawn Chance` CatapultSpawnChance)
  (set `self.Max Catapults` MaxCatapults)
  (`self.Countdown`)
  (`self.Spawn_Catapult`))

(event `Spawn_Catapult`
  (bind (_returnvalue_x _returnvalue_y _returnvalue_z) (`KismetMathLibrary.BreakVector` (`self.K2_GetActorLocation`)))
  ;[1 0.8413 0.08369] Checks time left
  (if (>= (`self.Wave_Time`) 0)
    (bind _outactors (`GameplayStatics.GetAllActorsWithTag` "Catapult"))
    (if (< (`KismetArrayLibrary.Array_Length` _outactors) (`self.Max Catapults`))
      (if (== (`self.Catapult Spawn Chance`) (`KismetMathLibrary.RandomIntegerInRange` 1 (`self.Catapult Spawn Chance`)))
        (`|SpawnActorFromClass` "/Game/0_Greyden_Content/AI/AI_Catapult.AI_Catapult_C" (`KismetMathLibrary.MakeTransform` (`KismetMathLibrary.MakeVector` (+ _returnvalue_x (`KismetMathLibrary.RandomIntegerInRange` -1500 1500)) (+ _returnvalue_y (`KismetMathLibrary.RandomIntegerInRange` -1500 1500)) _returnvalue_z)) "Undefined" "MultiplyWithRoot" null null)))
    (`KismetSystemLibrary.Delay` (`KismetMathLibrary.Conv_IntToDouble` (`KismetMathLibrary.RandomIntegerInRange` 20 30)))
    (`self.Spawn_Catapult`)
    (else
      (`self.Spawn_Catapult_Final`))))

(event `Spawn_Catapult_Final`
  (bind (_returnvalue_x _returnvalue_y _returnvalue_z) (`KismetMathLibrary.BreakVector` (`self.K2_GetActorLocation`)))
  (`KismetSystemLibrary.Delay` (`KismetMathLibrary.RandomFloatInRange` 0.0 0.5))
  (bind _outactors (`GameplayStatics.GetAllActorsWithTag` "Catapult"))
  (if (< (`KismetArrayLibrary.Array_Length` _outactors) (`self.Max Catapults`))
    (`|SpawnActorFromClass` "/Game/0_Greyden_Content/AI/AI_Catapult.AI_Catapult_C" (`KismetMathLibrary.MakeTransform` (`KismetMathLibrary.MakeVector` (+ _returnvalue_x (`KismetMathLibrary.RandomIntegerInRange` -1500 1500)) (+ _returnvalue_y (`KismetMathLibrary.RandomIntegerInRange` -1500 1500)) _returnvalue_z)) "Undefined" "MultiplyWithRoot" null null)))

(fn `UserConstructionScript`)