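; BP_Target is a target actor that reacts to being hit by actors tagged "Fireball".
; An overlap on either its static or skeletal mesh runs the same hit sequence.
; The sequence teleports the target down out of its position, sets the Demo flag on a referenced console, then teleports it back up after a fixed delay.
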(event `self.StaticMesh.OnComponentBeginOverlap`
  (params (OverlappedComponent :type "PrimitiveComponent Object Reference") (OtherActor :type "Actor Object Reference") (OtherComp :type "PrimitiveComponent Object Reference") (OtherBodyIndex :type Integer) (bFromSweep :type Boolean) (SweepResult :type "HitResult Structure (by ref)"))
  ;[1 0.4 0.01108] Hit by fire ball
  (if (`self.ActorHasTag` OtherActor "Fireball")
    (`self.K2_TeleportTo` (- (`self.K2_GetActorLocation`) (0.0 0.0 100.0)) (`self.K2_GetActorRotation`) :!label _label)
    (set `/Game/StartandEndLevels/console_BP.Demo` true (`self.Console_Ref`))
    (`KismetSystemLibrary.Delay` 7.0)
    (`self.K2_TeleportTo` (+ (`self.K2_GetActorLocation`) (0.0 0.0 100.0)) (`self.K2_GetActorRotation`))))

(event `self.SkeletalMesh.OnComponentBeginOverlap`
  (params (OverlappedComponent :type "PrimitiveComponent Object Reference") (OtherActor :type "Actor Object Reference") (OtherComp :type "PrimitiveComponent Object Reference") (OtherBodyIndex :type Integer) (bFromSweep :type Boolean) (SweepResult :type "HitResult Structure (by ref)"))
  (if (`self.ActorHasTag` OtherActor "Fireball")
    (goto _label)))

(fn `UserConstructionScript`)